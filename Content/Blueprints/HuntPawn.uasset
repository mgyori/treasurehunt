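; Player pawn for a hero card game, showing a hand of cards and a row of center cards as spawned CardActors.
; On non-server BeginPlay it rotates its root and registers with HuntController.
; Server/Client event pairs, gated by authority switches, add, remove or replace cards.
; Layout functions fan the hand around its midpoint and space scaled-down center cards in a row, all attached to Hand.
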(event Custom|Server_ReplaceAllCardFromCenter
  (params (NewHeroes :type Array%20of%20Integers))
  (Networking|SwitchHasAuthority
    (:Authority
      (CallFunction|ClientReplaceAllCardfromCenter NewHeroes)
      (bind _ashunt_controller (Utilities|Casting|CastToHuntController (Pawn|GetController)))
      (Variables|/Game/Blueprints/HuntController.HuntController_C|SetPlayerGameState _ashunt_controller 0))))

(event Custom|Server_AddCardToCenter
  (params (Hero :type Integer))
  (Networking|SwitchHasAuthority
    (:Remote
      (CallFunction|ClientAddCardtoCenter Hero))))

(event Custom|Client_AddCardToCenter
  (params (Hero :type Integer))
  (Networking|SwitchHasAuthority
    (:Remote
      (CallFunction|AddCardtoCenter Hero)
      (CallFunction|SetCenterCardPositions))))

(event Custom|Client_RemoveCardFromCenter
  (params (HeroID :type Integer))
  (bind _centercards (Variables|Default|GetCenterCards))
  (Networking|SwitchHasAuthority
    (:Remote
      (for _array_element _centercards
        (if (== (Variables|/Game/Blueprints/CardActor.CardActor_C|GetCardHero _array_element) HeroID)
          (Actor|DestroyActor _array_element)
          (Utilities|Array|RemoveItem _centercards _array_element)))
      (CallFunction|SetCenterCardPositions))))

(event Custom|Server_RemoveCardFromCenter
  (params (HeroID :type Integer))
  (Networking|SwitchHasAuthority
    (:Authority
      (CallFunction|ClientRemoveCardfromCenter HeroID)
      (Utilities|Array|RemoveItem (Variables|Default|GetServer_CenterCards) HeroID))))

(event Custom|Client_AddCardToHand
  (params (Hero :type Integer))
  (Networking|SwitchHasAuthority
    (:Remote
      (CallFunction|AddCardtoHand Hero)
      (CallFunction|SetCardPositions))))

(event Custom|Server_AddCardToHand
  (params (Hero :type Integer))
  (Networking|SwitchHasAuthority
    (:Authority
      (CallFunction|ClientAddCardtoHand Hero))))

(event Custom|Client_ReplaceAllCardFromCenter
  (params (NewHeroes :type Array%20of%20Integers))
  (bind _centercards (Variables|Default|GetCenterCards))
  (Networking|SwitchHasAuthority
    (:Remote
      (for _array_element _centercards
        (Actor|DestroyActor _array_element))
      (Utilities|Array|Clear _centercards)
      (for _array_element_2 NewHeroes
        (CallFunction|ClientAddCardtoCenter _array_element_2)))))

(event EventBeginPlay
  (bind _self self)
  (if (not (Networking|IsServer))
    (Transformation|SetWorldRotation (Variables|Default|GetDefaultSceneRoot) "-80.000000,-90.000000, 0" false false)
    (bind _ashunt_controller (Utilities|Casting|CastToHuntController (Pawn|GetController)))
    (Variables|/Game/Blueprints/HuntController.HuntController_C|SetOwnHuntPawn _ashunt_controller _self)
    (Default|OnReadyEvent _ashunt_controller _self)))

(fn ConstructionScript)

(fn AddCardtoHand
  (params (Hero :type Integer))
  (bind _returnvalue (Game|SpawnActorfromClass "/Game/Blueprints/CardActor.CardActor_C" (Math|Transform|MakeTransform "0.000000,-30.000000, 0" "0,180.000000, 0" "1,1,1") "Undefined" 0 0))
  (Variables|/Game/Blueprints/CardActor.CardActor_C|SetCardHero _returnvalue Hero)
  (Default|SetCardHero _returnvalue)
  (Transformation|AttachComponentToComponent _returnvalue (Variables|Default|GetHand) "Hand" "KeepRelative" "KeepRelative" "KeepRelative" false)
  (Utilities|Array|Add (Variables|Default|GetCards) _returnvalue))

(fn SetCardPositions
  (bind _cards (Variables|Default|GetCards))
  (bind _returnvalue (Utilities|Array|Length _cards))
  (bind _returnvalue_2 (Math|Conversions|ToFloat(Integer) _returnvalue))
  (bind _returnvalue_3 (/ _returnvalue_2 2.0))
  (bind _returnvalue_4 (Math|Float|Floor _returnvalue_3))
  (for (_array_element _array_index) _cards
    (if (> _array_index _returnvalue_4)
      (Transformation|SetRelativeLocation (Variables|/Game/Blueprints/CardActor.CardActor_C|GetCard _array_element) (Math|Vector|MakeVector (- (* _array_index 2e+01) (+ (* _returnvalue 1e+01) -2e+01)) (* _array_index 0.5) (* _array_index 0.5)) false false)
      (Transformation|SetRelativeRotation (Variables|/Game/Blueprints/CardActor.CardActor_C|GetCard _array_element) (Math|Rotator|MakeRotator 0.0 0.0 (* _array_index 1.0)) false false)
      (else
        (Transformation|SetRelativeLocation (Variables|/Game/Blueprints/CardActor.CardActor_C|GetCard _array_element) (Math|Vector|MakeVector (+ (- (* _array_index 2e+01) (+ (* _returnvalue 1e+01) -2e+01)) -28.0) (* (- _array_index _returnvalue_4) -0.5) (* (- _array_index _returnvalue_4) -0.5)) false false)
        (Transformation|SetRelativeRotation (Variables|/Game/Blueprints/CardActor.CardActor_C|GetCard _array_element) (Math|Rotator|MakeRotator 0.0 0.0 (* (- _array_index _returnvalue_4) 1.0)) false false)))))

(fn AddCardtoCenter
  (params (Hero :type Integer))
  (bind _returnvalue (Game|SpawnActorfromClass "/Game/Blueprints/CardActor.CardActor_C" (Math|Transform|MakeTransform "0.000000,-30.000000, 0" "0,180.000000, 0" "1,1,1") "Undefined" 0 0))
  (Variables|/Game/Blueprints/CardActor.CardActor_C|SetCardHero _returnvalue Hero)
  (Variables|/Game/Blueprints/CardActor.CardActor_C|SetCenterCard _returnvalue true)
  (Default|SetCardHero _returnvalue)
  (Transformation|AttachComponentToComponent _returnvalue (Variables|Default|GetHand) "Hand" "KeepRelative" "KeepRelative" "KeepRelative" false)
  (Utilities|Array|Add (Variables|Default|GetCenterCards) _returnvalue))

(fn SetCenterCardPositions
  (bind _centercards (Variables|Default|GetCenterCards))
  (for (_array_element _array_index) _centercards
    (Transformation|SetRelativeLocation (Variables|/Game/Blueprints/CardActor.CardActor_C|GetCard _array_element) (Math|Vector|MakeVector (- (* _array_index 6e+01) (+ (* (Utilities|Array|Length _centercards) 3e+01) -3e+01)) -1.8e+02 0.0) false false)
    (Transformation|SetActorScale3D (Components|GetOwner (Variables|/Game/Blueprints/CardActor.CardActor_C|GetCard _array_element)) "0.500000,0.500000,1.000000")))