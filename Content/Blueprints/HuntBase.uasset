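; Game mode for the Hunt game that registers joining players and sets up a random board of treasure cards and goblins.
; PostLogin assigns each player an incrementing ID; once enough ready reports arrive, OnLoaded notifies every HuntController and calls LoadRandomBoard inside that per-controller loop.
; Board setup gives each TreasureCard an unused material-based index by retrying random picks, then randomizes each Goblin's paw, gold and goblin values.
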(event Custom|Server_OnPlayerReadyEvent
  (params (PlayerID :type Integer))
  (Development|PrintString (Utilities|String|Append "Betöltve: " (Utilities|String|ToString(Integer) PlayerID)))
  (bind _output_get (Variables|Default|SetReadyPlayers (+ (Variables|Default|GetReadyPlayers) 1)))
  (if (>= _output_get (Utilities|Array|Length (Variables|Default|GetPlayers)))
    (CallFunction|OnLoaded)))

(event Custom|OnLoaded
  (Development|PrintString "LOADED!" true true "(R=0.113357,G=1.000000,B=0.000000,A=1.000000)" 5.0)
  (bind _outactors (Actor|GetAllActorsOfClass "/Game/Blueprints/HuntController.HuntController_C"))
  (for _array_element _outactors
    (Default|OnLoaded _array_element (Variables|/Game/Blueprints/HuntController.HuntController_C|GetMyID _array_element))
    (CallFunction|LoadRandomBoard)))

(event Custom|LoadRandomBoard
  (bind _treasurecardsintable (Variables|Default|GetTreasureCardsInTable))
  (bind _outactors (Actor|GetAllActorsOfClass "/Game/Blueprints/TreasureCard.TreasureCard_C"))
  (for _array_element _outactors
    (bind _number (CallFunction|GetRandomTresureCard _array_element :!label _label))
    (if (Utilities|Array|ContainsItem _treasurecardsintable _number)
      (goto _label)
      (else
        (Utilities|Array|AddUnique _treasurecardsintable _number)
        (Default|SetTreasureIndex _array_element _number))))
  (bind _outactors_2 (Actor|GetAllActorsOfClass "/Game/Blueprints/Goblin.Goblin_C"))
  (for _array_element_2 _outactors_2
    (Default|ServerSetGoblinData _array_element_2 (Math|Random|RandomIntegerinRange 1 3) (Math|Random|RandomIntegerinRange 1 3) (Math|Random|RandomInteger 2))))

(event EventPostLogin
  (params (NewPlayer :type Player%20Controller%20Object%20Reference))
  (if (Networking|IsServer)
    (bind _ashunt_player_state (Utilities|Casting|CastToHuntPlayerState (Variables|/Script/Engine.Controller|GetPlayerState NewPlayer)))
    (bind _output_get (Variables|Default|SetLastPlayerID (+ (Variables|Default|GetLastPlayerID) 1)))
    (Variables|/Game/Blueprints/HuntPlayerState.HuntPlayerState_C|SetTestID _ashunt_player_state _output_get)
    (bind _ashunt_controller (Utilities|Casting|CastToHuntController NewPlayer))
    (Utilities|Array|Add (Variables|Default|GetPlayers) _ashunt_controller)
    (Default|ServerSetID _ashunt_controller _output_get)))

(fn ConstructionScript)

(fn GetRandomTresureCard
  (params (Card :type Treasure%20Card%20Object%20Reference))
  (return (Math|Random|RandomInteger (Utilities|Array|Length (Rendering|Material|GetMaterials (Variables|/Game/Blueprints/TreasureCard.TreasureCard_C|GetCard Card))))))