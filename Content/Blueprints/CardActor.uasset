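; CardActor is a clickable hero card that a player's HuntPawn holds in the Hunt game, with its material picked by CardHero index.
; A click in game state 0 calls a client event that removes and destroys the card and re-lays out the pawn's cards, then multicasts state 1 through HuntState.
; Other states print a wrong-phase message in Hungarian.
; Cursor hover either scales or offsets the card, depending on ScaleHover.
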(event OnBeginCursorOver(Card)
  (params (TouchedComponent :type Primitive%20Component%20Object%20Reference))
  (if (Variables|Default|GetScaleHover)
    (Transformation|SetWorldScale3D TouchedComponent "0.302500,0.429000,1.000000")
    (else
      (Transformation|AddWorldOffset TouchedComponent "0,-40.000000,10.000000" false false))))

(event OnEndCursorOver(Card)
  (params (TouchedComponent :type Primitive%20Component%20Object%20Reference))
  (if (Variables|Default|GetScaleHover)
    (Transformation|SetWorldScale3D TouchedComponent "0.275000,0.390000,1.000000")
    (else
      (Transformation|AddWorldOffset TouchedComponent "0,40.000000,-10.000000" false false))))

(event OnClicked(Card)
  (params (TouchedComponent :type Primitive%20Component%20Object%20Reference) (ButtonPressed :type Key%20Structure :default "None"))
  (bind _ashunt_state (Utilities|Casting|CastToHuntState (Game|GetGameState)))
  (if (== (Variables|/Game/Blueprints/HuntState.HuntState_C|GetGameStateVar _ashunt_state) 0)
    (CallFunction|ClientRemoveCard TouchedComponent)
    (Default|MulticastSetGameState _ashunt_state 1)
    (else
      (Development|PrintString "Jelenleg nem ez a fázis van mo!"))))

(event Custom|SetCardHero
  (Rendering|Material|SetMaterial (Variables|Default|GetCard) 0 (Utilities|Array|Get(acopy) (Rendering|Material|GetMaterials (Variables|Default|GetCard)) (Variables|Default|GetCardHero))))

(event Custom|Client_RemoveCard
  (params (Actor :type Actor%20Component%20Object%20Reference))
  (bind _returnvalue (Components|GetOwner Actor))
  (bind _ashunt_pawn (Utilities|Casting|CastToHuntPawn (Game|Player|GetPlayerPawn 0)))
  (bind _ascard_actor (Utilities|Casting|CastToCardActor _returnvalue))
  (Utilities|Array|RemoveItem (Variables|/Game/Blueprints/HuntPawn.HuntPawn_C|GetCards _ashunt_pawn) _ascard_actor)
  (Actor|DestroyActor _returnvalue)
  (Default|SetCardPositions _ashunt_pawn))

(fn ConstructionScript
  (Rendering|Material|SetMaterial (Variables|Default|GetCard) 0 (Utilities|Array|Get(acopy) (Rendering|Material|GetMaterials (Variables|Default|GetCard)) (Variables|Default|GetCardHero))))