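; Player controller for the Hunt mode that holds a player ID and reports the player as ready to the server.
; Client_SetID stores the assigned ID, and BeginPlay on the remote side calls a server event.
; That event passes the server's copy of MyID to the HuntBase game mode's ready event.
; Logic to copy the ID into HuntUI widgets is present but never runs.
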(event Custom|Client_SetID
  (params (ID :type Integer))
  (Variables|Default|SetMyID ID))

(event Custom|Server_Try
  (bind _ashunt_base (Utilities|Casting|CastToHuntBase (Game|GetGameMode)))
  (Default|ServeronPlayerReadyEvent _ashunt_base (Variables|Default|GetMyID)))

(event EventBeginPlay
  (Networking|SwitchHasAuthority
    (:Remote
      (CallFunction|ServerTry))))

(event EventTick
  (params (DeltaSeconds :type Float%20%28single-precision%29)))

(fn ConstructionScript)