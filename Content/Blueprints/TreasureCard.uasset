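; TreasureCard is a card actor whose face shows the treasure selected by TreasureIndex.
; The construction script copies the Card component's material at that index into slot 0, so the component's material slots double as the lookup table.
; SetTreasureIndex multicasts directly on authority or routes through a server event otherwise; the multicast stores the index, reapplies the material and prints a leftover debug string.
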(event Custom|Multicast_SetTreasureIndex
  (params (Index :type Integer))
  (Variables|Default|SetTreasureIndex Index)
  (Rendering|Material|SetMaterial (Variables|Default|GetCard) 0 (Rendering|Material|GetMaterial (Variables|Default|GetCard) (Variables|Default|GetTreasureIndex)))
  (Development|PrintString "asasd"))

(event Custom|Server_SetTreasureIndex
  (params (Index :type Integer))
  (CallFunction|MulticastSetTreasureIndex Index))

(event Custom|SetTreasureIndex
  (params (Index :type Integer))
  (Networking|SwitchHasAuthority
    (:Authority
      (CallFunction|MulticastSetTreasureIndex Index))
    (:Remote
      (CallFunction|ServerSetTreasureIndex Index))))

(event EventBeginPlay)

(event Collision|EventActorBeginOverlap
  (params (OtherActor :type Actor%20Object%20Reference)))

(event EventTick
  (params (DeltaSeconds :type Float%20%28single-precision%29)))

(fn ConstructionScript
  (Rendering|Material|SetMaterial (Variables|Default|GetCard) 0 (Rendering|Material|GetMaterial (Variables|Default|GetCard) (Variables|Default|GetTreasureIndex))))